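; Interactable pickup item that shows a "Press E to Pick Item" prompt and provides events for collecting it.
; Additemtoinventory casts to the first-person character and adds the item's ID and name to its inventory component.
; A successful add optionally destroys the actor, while a failed one prints that the item is already owned.
; A separate PlaySound event spawns positional audio, using an optional attenuation override or the default setting.
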(event Custom|Add%20item%20to%20inventory
  (params (New%20Item%20Item%20ID :type String) (New%20Item%20Item%20Name :type Name) (Destroy%20Actor%20After%20Adding%20To%20Inventory :type Boolean))
  ;[0.15 0.15 0.15 0.5] Add item to inventory
  (bind _asbp_first_person_character (Utilities|Casting|CastToBP_FirstPersonCharacter (Game|GetPlayerCharacter 0)))
  (bind _added (Default|AddItem (Variables|/Game/FirstPerson/Blueprints/BP_FirstPersonCharacter.BP_FirstPersonCharacter_C|GetBP_InventoryComponent _asbp_first_person_character) (Utilities|Struct|MakeItemStruct New%20Item%20Item%20ID New%20Item%20Item%20Name)))
  (if _added
    (if Destroy%20Actor%20After%20Adding%20To%20Inventory
      (Actor|DestroyActor))
    (else
      (Development|PrintString "You already have this item"))))

(event Custom|Play%20Sound
  (params (Sound :type Sound%20Base%20Object%20Reference) (Location :type Vector) (Attenuation%20OPT. :type Sound%20Attenuation%20Object%20Reference))
  ;[0.15 0.15 0.15 0.5] Play Sound
  (Utilities|IsValid Sound
    (:Is%20Valid
      (Utilities|IsValid Attenuation%20OPT.
        (:Is%20Valid
          (Audio|SpawnSoundatLocation Sound Location "0, 0, 0" 1.0 1.0 0.0 Attenuation%20OPT. 0))
        (:Is%20Not%20Valid
          (Audio|SpawnSoundatLocation Sound Location "0, 0, 0" 1.0 1.0 0.0 (Variables|Default|GetAttenuation%20Settings) 0))))
    (:Is%20Not%20Valid
      (Utilities|IsValid Attenuation%20OPT.
        (:Is%20Valid
          (Audio|SpawnSoundatLocation (Variables|Default|GetSound) "0, 0, 0" "0, 0, 0" 1.0 1.0 0.0 Attenuation%20OPT. 0))
        (:Is%20Not%20Valid
          (Audio|SpawnSoundatLocation (Variables|Default|GetSound) Location "0, 0, 0" 1.0 1.0 0.0 (Variables|Default|GetAttenuation%20Settings) 0))))))

(event EventBeginPlay
  (|CallParentFunction)
  ;[0.15 0.15 0.15 0.5] Custom Interaction Text
  (CallFunction|SetInteractionText "Press E to Pick Item"))

(fn ConstructionScript
  (|CallParentFunction))