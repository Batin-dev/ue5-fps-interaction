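; Base Blueprint for interactable pickup items, which sets a "Press E to Pick" prompt on BeginPlay.
; AddItemToInventory caches the first-person player character, passes the item's ID, name and uniqueness to its inventory component, and returns success.
; DestroyActorSafe destroys the item and hides that cached character's interaction widget.
; A PlaySound event spawns sound at a location, using optional attenuation or the default settings.
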(event Custom|Play%20Sound
  (params (Sound :type Sound%20Base%20Object%20Reference) (Location :type Vector) (Attenuation%20OPT. :type Sound%20Attenuation%20Object%20Reference))
  ;[0.15 0.15 0.15 0.5] Play Sound
  (Utilities|IsValid Sound
    (:Is%20Valid
      (Utilities|IsValid Attenuation%20OPT.
        (:Is%20Valid
          (Audio|SpawnSoundatLocation Sound Location "0, 0, 0" 1.0 1.0 0.0 Attenuation%20OPT. 0))
        (:Is%20Not%20Valid
          (Audio|SpawnSoundatLocation Sound Location "0, 0, 0" 1.0 1.0 0.0 (Variables|Default|GetAttenuation%20Settings) 0))))
    (:Is%20Not%20Valid
      (Utilities|IsValid Attenuation%20OPT.
        (:Is%20Valid
          (Audio|SpawnSoundatLocation (Variables|Default|GetSound) "0, 0, 0" "0, 0, 0" 1.0 1.0 0.0 Attenuation%20OPT. 0))
        (:Is%20Not%20Valid
          (Audio|SpawnSoundatLocation (Variables|Default|GetSound) Location "0, 0, 0" 1.0 1.0 0.0 (Variables|Default|GetAttenuation%20Settings) 0))))))

(event EventBeginPlay
  (|CallParentFunction)
  ;[0.15 0.15 0.15 0.5] Custom Interaction Text
  (CallFunction|SetInteractionText "Press E to Pick"))

(fn ConstructionScript
  (|CallParentFunction))

(fn AddItemtoInventory
  (params (Item%20ID :type String) (Item%20Name :type Name) (Is%20Unique :type Boolean))
  (bind _asbp_first_person_character (Utilities|Casting|CastToBP_FirstPersonCharacter (Game|GetPlayerCharacter 0)))
  (bind _output_get (Variables|Default|SetAs%20BP%20First%20Person%20Character _asbp_first_person_character))
  (bind _added (Default|AddItem (Variables|/Game/BP/Character/BP_FirstPersonCharacter.BP_FirstPersonCharacter_C|GetBP_InventoryComponent _output_get) (Utilities|Struct|MakeItemStruct Item%20ID Item%20Name Is%20Unique)))
  (if _added
    (return true)
    (else
      (return false))))

(fn DestroyActor(Safe)
  (Actor|DestroyActor)
  (Default|Hide (Variables|/Game/BP/Character/BP_FirstPersonCharacter.BP_FirstPersonCharacter_C|GetInteractionWidget (Variables|Default|GetAs%20BP%20First%20Person%20Character))))