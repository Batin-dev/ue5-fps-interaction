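; Base Blueprint for interactable actors, providing outline highlighting, settable interaction text and a placeholder Interact event that only prints a debug string.
; On BeginPlay it gathers its static mesh components, skipping any tagged NoOutline, and enables custom depth rendering on them.
; ActiveOutline and DeActiveOutline toggle the highlight by switching those meshes' custom depth stencil value, guarded by a state flag.
; SetInteractionText stores the supplied text only when it is not empty.
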(event Custom|DeActiveOutline
  ;[0.15 0.15 0.15 0.5] Outline
  (if (Variables|Default|GetIsOutlineActive)
    (Variables|Default|SetIsOutlineActive false)
    (for _array_element (Variables|Default|GetHighlight%20Meshes)
      (Rendering|SetCustomDepthStencilValue _array_element 0))))

(event Custom|ActiveOutline
  ;[0.15 0.15 0.15 0.5] Outline
  (if (not (Variables|Default|GetIsOutlineActive))
    (Variables|Default|SetIsOutlineActive true)
    (for _array_element (Variables|Default|GetHighlight%20Meshes)
      (Rendering|SetCustomDepthStencilValue _array_element 1))))

(event EventBeginPlay
  (CallFunction|PrepareOutlineMeshes (Variables|Default|GetHighlight%20Meshes)))

(event EventInteract
  (Development|PrintString "Hey I'm literally empty"))

(fn ConstructionScript)

(fn PrepareOutlineMeshes
  (params (Highlight%20Meshes :type Array%20of%20Static%20Mesh%20Component%20Object%20References))
  (bind _returnvalue (Actor|GetComponentsByClass "/Script/Engine.StaticMeshComponent"))
  (if (Utilities|Array|IsNotEmpty _returnvalue)
    (for _array_element _returnvalue
      (if (not (Components|ComponentHasTag _array_element "NoOutline"))
        (Utilities|Array|Add Highlight%20Meshes _array_element)
        (Rendering|SetRenderCustomDepth _array_element true)))))

(fn SetInteractionText
  (params (Text :type Text))
  (if (not (Utilities|Text|TextIsEmpty Text))
    (Variables|Default|SetInteractionText Text)))