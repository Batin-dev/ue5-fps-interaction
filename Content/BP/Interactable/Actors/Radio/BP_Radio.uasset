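; BP_Radio is an interactable radio actor that the player toggles on and off.
; Interact spawns an attenuated sound at the RadioBase location, or stops the stored audio component after a short delay, updating the playing flag and interaction prompt.
; On BeginPlay, InitializeActor reuses the turn-on branch, so a radio with IsPlaying set starts out playing.
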(event Custom|InitializeActor
  (params (Is%20Playing :type Boolean))
  (if Is%20Playing
    (bind _returnvalue (Audio|SpawnSoundatLocation (Variables|Default|GetSound) (Transformation|GetWorldLocation (Variables|Default|GetRadioBase)) "0, 0, 0" 1.0 1.0 0.0 (Variables|Default|GetAttenuation%20Settings) 0))
    (CallFunction|SetInteractionText "Press E to Turn the Radio Off")
    (Variables|Default|SetIsPlaying true)))

(event EventBeginPlay
  (|CallParentFunction)
  ;[0.15 0.15 0.15 0.5] Custom Interaction Text
  (CallFunction|SetInteractionText "Press E to Turn the Radio On")
  ;[0.15 0.15 0.15 0.5] Set Ready Effects In Start
  (CallFunction|InitializeActor (Variables|Default|GetIsPlaying)))

(event Collision|EventActorBeginOverlap
  (params (OtherActor :type Actor%20Object%20Reference)))

(event EventTick
  (params (DeltaSeconds :type Float%20%28single-precision%29)))

(event EventInteract
  (if (Variables|Default|GetIsPlaying)
    (Utilities|IsValid (stale _returnvalue)
      (:Is%20Valid
        (Utilities|FlowControl|Delay 0.35)
        (Audio|Components|Audio|Stop (stale _returnvalue))
        (Variables|Default|SetIsPlaying false)
        (CallFunction|SetInteractionText "Press E to Turn the Radio On")))
    (else
      (bind _returnvalue (Audio|SpawnSoundatLocation (Variables|Default|GetSound) (Transformation|GetWorldLocation (Variables|Default|GetRadioBase)) "0, 0, 0" 1.0 1.0 0.0 (Variables|Default|GetAttenuation%20Settings) 0))
      (CallFunction|SetInteractionText "Press E to Turn the Radio Off")
      (Variables|Default|SetIsPlaying true))))

(fn ConstructionScript
  (|CallParentFunction))