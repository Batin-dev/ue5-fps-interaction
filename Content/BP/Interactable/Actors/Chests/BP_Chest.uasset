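; Interactable chest that the player opens and closes, with the interaction prompt switching between open and close text.
; Interact plays or reverses OpenCloseTL, whose alpha drives the BoxLid roll rotation.
; A sound plays as opening starts, or after a timeline-length delay when closing.
; CanOpen blocks further interaction until a short delay after the sound, when the prompt updates.
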(event EventBeginPlay
  (|CallParentFunction)
  (CallFunction|SetInteractionText "Press E to Open"))

(event Collision|EventActorBeginOverlap
  (params (OtherActor :type Actor%20Object%20Reference)))

(event EventTick
  (params (DeltaSeconds :type Float%20%28single-precision%29)))

(event EventInteract
  (bind _attenuation_settings (Variables|Default|GetAttenuation%20Settings))
  (if (Variables|Default|GetCanOpen)
    (if (Variables|Default|GetIsOpened)
      (Variables|Default|SetIsOpened false)
      (Variables|Default|SetCanOpen false)
      (Utilities|FlowControl|Sequence
        (:then_0
          (Utilities|FlowControl|Delay (Components|Timeline|GetTimelineLength (Variables|Default|GetOpenCloseTl)))
          (Audio|PlaySoundatLocation "/Engine/EditorSounds/GamePreview/PossessPlayer_Cue.PossessPlayer_Cue" "0, 0, 0" "0, 0, 0" 1.0 1.0 0.0 _attenuation_settings 0 0 0)
          (Utilities|FlowControl|Delay 0.5)
          (CallFunction|SetInteractionText "Press E to Open")
          (Variables|Default|SetCanOpen true :!label _label))
        (:then_1
          (bind _alpha (Timeline|OpenCloseTL Reverse)
            (:Update
              (Transformation|SetRelativeRotation (Variables|Default|Getbox%20lid) (Math|Rotator|MakeRotator (Math|Float|Lerp 0.0 1.1e+02 _alpha) 0.0 0.0) false false)))))
      (else
        (Variables|Default|SetIsOpened true)
        (Variables|Default|SetCanOpen false)
        (Utilities|FlowControl|Sequence
          (:then_0
            (Timeline|OpenCloseTL Play))
          (:then_1
            (Audio|PlaySoundatLocation "/Engine/EditorSounds/GamePreview/PossessPlayer_Cue.PossessPlayer_Cue" "0, 0, 0" "0, 0, 0" 1.0 1.0 0.0 _attenuation_settings 0 0 0)
            (Utilities|FlowControl|Delay 0.5)
            (CallFunction|SetInteractionText "Press E to Close")
            (goto _label)))))))

(fn ConstructionScript
  (|CallParentFunction))