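; BP_BurnBarrel is an interactable burn barrel that the player ignites or extinguishes, optionally starting lit via IsBurning.
; Igniting spawns an emitter at the Fire component, then a delayed fire sound at world origin, and Interact shares this path with InitializeActor.
; Extinguishing deactivates the emitter, then stops the sound and clears IsBurning only if that sound is valid.
; Prompts follow the state, but an initially unlit barrel keeps BeginPlay's "Turn the Radio On" text.
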(event Custom|InitializeActor
  (params (Is%20Burning :type Boolean))
  (if Is%20Burning
    ;[0.15 0.15 0.15 0.5] Interaction Override
    (bind _returnvalue (Effects|SpawnEmitteratLocation (Variables|Default|GetEmitter%20Template) (Transformation|GetWorldLocation (Variables|Default|Getfire)) "0, 0, 0" "0.800000,1.000000,1.000000"))
    (CallFunction|SetInteractionText "Press E to Extinguish")
    (Utilities|FlowControl|Delay 0.4)
    (bind _returnvalue_2 (Audio|SpawnSoundatLocation "/Game/StarterContent/Audio/Fire01_Cue.Fire01_Cue" "0, 0, 0" "0, 0, 0" 1.0 1.0 0.0 0 0))
    (Variables|Default|SetIsBurning true)))

(event EventBeginPlay
  (|CallParentFunction)
  ;[0.15 0.15 0.15 0.5] Custom Interaction Text
  (CallFunction|SetInteractionText "Press E to Turn the Radio On")
  ;[0.15 0.15 0.15 0.5] Set Ready Effects In Start
  (CallFunction|InitializeActor (Variables|Default|GetIsBurning)))

(event Collision|EventActorBeginOverlap
  (params (OtherActor :type Actor%20Object%20Reference))
  (|CallParentFunction OtherActor) ; This node is disabled and will not be called.\nDrag off pins to build functionality.
)

(event EventTick
  (params (DeltaSeconds :type Float%20%28single-precision%29))
  (|CallParentFunction DeltaSeconds) ; This node is disabled and will not be called.\nDrag off pins to build functionality.
)

(event EventInteract
  ;[0.15 0.15 0.15 0.5] Interaction Override
  (if (Variables|Default|GetIsBurning)
    (Components|Activation|Deactivate (stale _returnvalue))
    (CallFunction|SetInteractionText "Press E to Ignite")
    (Utilities|IsValid (stale _returnvalue_2)
      (:Is%20Valid
        (Utilities|FlowControl|Delay 0.2)
        (Audio|Components|Audio|Stop (stale _returnvalue_2))
        (Variables|Default|SetIsBurning false)))
    (else
      (bind _returnvalue (Effects|SpawnEmitteratLocation (Variables|Default|GetEmitter%20Template) (Transformation|GetWorldLocation (Variables|Default|Getfire)) "0, 0, 0" "0.800000,1.000000,1.000000"))
      (CallFunction|SetInteractionText "Press E to Extinguish")
      (Utilities|FlowControl|Delay 0.4)
      (bind _returnvalue_2 (Audio|SpawnSoundatLocation "/Game/StarterContent/Audio/Fire01_Cue.Fire01_Cue" "0, 0, 0" "0, 0, 0" 1.0 1.0 0.0 0 0))
      (Variables|Default|SetIsBurning true))))

(fn ConstructionScript
  (|CallParentFunction))