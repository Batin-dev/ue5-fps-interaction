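; BP_Bonfire is an interactable bonfire that the player ignites and extinguishes.
; The Interact override uses a FlipFlop to alternate states and update the prompt text.
; Igniting spawns fire and smoke emitters at the Fire component, then starts the sound and shows the point light after a short delay.
; Extinguishing deactivates the emitters and, only if the sound is valid, stops it and hides the light after a delay.
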(event EventBeginPlay
  (|CallParentFunction)
  ;[0.15 0.15 0.15 0.5] Custom Interaction Text
  (CallFunction|SetInteractionText "Press E to Ignite"))

(event Collision|EventActorBeginOverlap
  (params (OtherActor :type Actor%20Object%20Reference))
  (|CallParentFunction OtherActor) ; This node is disabled and will not be called.\nDrag off pins to build functionality.
)

(event EventTick
  (params (DeltaSeconds :type Float%20%28single-precision%29))
  (|CallParentFunction DeltaSeconds) ; This node is disabled and will not be called.\nDrag off pins to build functionality.
)

(event EventInteract
  (bind _fire (Variables|Default|Getfire))
  (bind _pointlight (Variables|Default|GetPointLight))
  (bind _returnvalue (Transformation|GetWorldLocation _fire))
  ;[0.15 0.15 0.15 0.5] Interaction Override
  (Utilities|FlowControl|FlipFlop
    (:A
      (bind _returnvalue_2 (Effects|SpawnEmitteratLocation "/Game/StarterContent/Particles/P_Fire.P_Fire" _returnvalue "0, 0, 0" "0.800000,1.000000,1.000000"))
      (bind _returnvalue_3 (Effects|SpawnEmitteratLocation "/Game/StarterContent/Particles/P_Smoke.P_Smoke" _returnvalue))
      (CallFunction|SetInteractionText "Press E to Extinguish")
      (Utilities|FlowControl|Delay 0.4)
      (bind _returnvalue_4 (Audio|SpawnSoundatLocation "/Game/StarterContent/Audio/Fire01_Cue.Fire01_Cue" _returnvalue "0, 0, 0" 1.0 1.0 0.0 0 0))
      (Rendering|SetVisibility _pointlight true false))
    (:B
      (Components|Activation|Deactivate _returnvalue_2)
      (Components|Activation|Deactivate _returnvalue_3)
      (CallFunction|SetInteractionText "Press E to Ignite")
      (Utilities|IsValid _returnvalue_4
        (:Is%20Valid
          (Utilities|FlowControl|Delay 0.2)
          (Audio|Components|Audio|Stop _returnvalue_4)
          (Rendering|SetVisibility _pointlight false false))))))

(fn ConstructionScript
  (|CallParentFunction))