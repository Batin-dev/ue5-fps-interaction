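; BP_Interactable_Base_Child2 is a child interactable actor that changes its cube's color when the player interacts with it.
; On BeginPlay it runs the parent logic and sets the prompt to "Press E to Change Color".
; Its Interact override uses a FlipFlop to alternate the Cube mesh's first material slot between two materials on each interaction.
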(event EventBeginPlay
  (|CallParentFunction)
  (CallFunction|SetInteractionText "Press E to Change Color"))

(event Collision|EventActorBeginOverlap
  (params (OtherActor :type Actor%20Object%20Reference))
  (|CallParentFunction OtherActor) ; This node is disabled and will not be called.\nDrag off pins to build functionality.
)

(event EventTick
  (params (DeltaSeconds :type Float%20%28single-precision%29))
  (|CallParentFunction DeltaSeconds) ; This node is disabled and will not be called.\nDrag off pins to build functionality.
)

(event EventInteract
  (bind _cube (Variables|Default|GetCube))
  ;[0.15 0.15 0.15 0.5] Interaction Override
  (Utilities|FlowControl|FlipFlop
    (:A
      (Rendering|Material|SetMaterial _cube 0 "/Engine/MapTemplates/Materials/BasicAsset03.BasicAsset03"))
    (:B
      (Rendering|Material|SetMaterial _cube 0 "/Engine/BasicShapes/BasicShapeMaterial.BasicShapeMaterial"))))

(fn ConstructionScript
  (|CallParentFunction))