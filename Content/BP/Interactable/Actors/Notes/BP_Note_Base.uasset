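; Base interactable note actor that lets the player read its text when they interact with it.
; It sets a "Press E to Read" prompt on begin play.
; On interact it plays a pickup sound, disables player character input, shows the mouse cursor and opens a WBP_Note widget carrying the note text.
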(event EventBeginPlay
  (|CallParentFunction)
  (CallFunction|SetInteractionText "Press E to Read"))

(event EventInteract
  ;[0.15 0.15 0.15 0.5] Sorry, this one isn’t modular :C
  (Audio|PlaySound2D (Variables|Default|GetPickSound) 1.0 1.0 0.0 0 0)
  (CallFunction|OpenNoteWidget (Variables|Default|GetNote%20Text)))

(fn ConstructionScript
  (|CallParentFunction))

(fn OpenNoteWidget
  (params (NoteText :type Text))
  (bind _returnvalue (Game|GetPlayerController 0))
  (Input|DisableInput (Game|GetPlayerCharacter 0) _returnvalue)
  (Variables|/Script/Engine.PlayerController|SetbShowMouseCursor _returnvalue true)
  (bind _returnvalue_2 (UserInterface|CreateWidget "/Game/UI/Notes/WBP_Note.WBP_Note_C" 0 NoteText))
  (bind _output_get (Variables|Default|SetNoteWidget _returnvalue_2))
  (UserInterface|Viewport|AddtoViewport _output_get 0))