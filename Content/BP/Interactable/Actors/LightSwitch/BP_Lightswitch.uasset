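; Interactable wall light switch that turns an assigned array of lights on and off.
; The Interact override flips IsOpened, tilts the Switch, plays the click sound at world origin with attenuation, then after a short delay sets each light component's visibility and updates the prompt.
; BeginPlay syncs switch rotation and prompt to IsOpened but leaves the lights' initial visibility untouched.
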(event Custom|InitializeActor
  (bind _switch (Variables|Default|GetSwitch))
  ;[0.15 0.15 0.15 0.5] Fix rotation
  (if (Variables|Default|GetIsOpened)
    (Transformation|SetRelativeRotation _switch (Math|Rotator|MakeRotator 5.0 0.0 0.0) false false)
    (CallFunction|SetInteractionText "Press E to Turn Off")
    (else
      (Transformation|SetRelativeRotation _switch (Math|Rotator|MakeRotator -5.0 0.0 0.0) false false)
      (CallFunction|SetInteractionText "Press E to Turn On"))))

(event EventBeginPlay
  (|CallParentFunction)
  (CallFunction|InitializeActor))

(event Collision|EventActorBeginOverlap
  (params (OtherActor :type Actor%20Object%20Reference))
  (|CallParentFunction OtherActor) ; This node is disabled and will not be called.\nDrag off pins to build functionality.
)

(event EventTick
  (params (DeltaSeconds :type Float%20%28single-precision%29))
  (|CallParentFunction DeltaSeconds) ; This node is disabled and will not be called.\nDrag off pins to build functionality.
)

(event EventInteract
  (bind _lights (Variables|Default|GetLights))
  (bind _attenuation_settings (Variables|Default|GetAttenuation%20Settings))
  (bind _switch (Variables|Default|GetSwitch))
  ;[0.15 0.15 0.15 0.5] Interaction Override
  (if (Variables|Default|GetIsOpened)
    (Variables|Default|SetIsOpened false)
    ;;[0.15 0.15 0.15 0.5] Close
    (Transformation|SetRelativeRotation _switch (Math|Rotator|MakeRotator -5.0 0.0 0.0) false false)
    (Audio|PlaySoundatLocation "/Game/Audio/LightSwitch/LightSwitch_Cue.LightSwitch_Cue" "0, 0, 0" "0, 0, 0" 1.0 1.0 0.0 _attenuation_settings 0 0 0)
    (Utilities|FlowControl|Delay 0.15)
    (for _array_element _lights
      (Rendering|SetVisibility (Variables|/Script/Engine.Light|GetLightComponent _array_element) false false))
    (CallFunction|SetInteractionText "Press E to Turn On")
    (else
      (Variables|Default|SetIsOpened true)
      ;;[0.15 0.15 0.15 0.5] Open
      (Transformation|SetRelativeRotation _switch (Math|Rotator|MakeRotator 5.0 0.0 0.0) false false)
      (Audio|PlaySoundatLocation "/Game/Audio/LightSwitch/LightSwitch_Cue.LightSwitch_Cue" "0, 0, 0" "0, 0, 0" 1.0 1.0 0.0 _attenuation_settings 0 0 0)
      (Utilities|FlowControl|Delay 0.15)
      (for _array_element_2 _lights
        (Rendering|SetVisibility (Variables|/Script/Engine.Light|GetLightComponent _array_element_2) true false))
      (CallFunction|SetInteractionText "Press E to Turn Off"))))

(fn ConstructionScript
  (|CallParentFunction))