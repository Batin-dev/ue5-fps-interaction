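; BP_Door_Child2 is a child door Blueprint that configures a specific door variant on top of its parent's logic.
; On BeginPlay it runs the parent setup, then sets the timeline play rate, open angle and open/close sounds, with a short delay on the close sound.
; All door behavior comes from the parent class; overlap and tick events are unused.
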(event EventBeginPlay
  (|CallParentFunction)
  ;[0.15 0.15 0.15 0.5] Door Settings
  (CallFunction|SetTLPlayRate 5.0)
  (CallFunction|SetOpenandCloseSounds "/Game/Audio/Doors/doorOpen2.doorOpen2" "/Game/Audio/Doors/doorClose2.doorClose2")
  (CallFunction|SetOpenAngle 1.2e+02)
  ;;[0.15 0.15 0.15 0.5] Optional
  (CallFunction|SetCloseSoundDelay 0.09))

(event Collision|EventActorBeginOverlap
  (params (OtherActor :type Actor%20Object%20Reference))
  (|CallParentFunction OtherActor) ; This node is disabled and will not be called.\nDrag off pins to build functionality.
)

(event EventTick
  (params (DeltaSeconds :type Float%20%28single-precision%29))
  (|CallParentFunction DeltaSeconds) ; This node is disabled and will not be called.\nDrag off pins to build functionality.
)

(fn ConstructionScript
  (|CallParentFunction))