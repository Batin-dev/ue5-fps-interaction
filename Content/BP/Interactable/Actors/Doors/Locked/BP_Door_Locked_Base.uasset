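; Base locked door actor that requires a key item from the player's inventory before it opens or closes.
; BeginPlay caches the inventory component from the first-person character.
; TryOpenDoor checks KeyID while locked, playing a jiggle or default locked sound when the key is missing.
; With the key, it blocks further attempts for the unlock sound's duration, then clears the lock and calls OpenCloseDoor.
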(event Custom|TryOpenDoor
  (params (Jiggle%20Sound :type Sound%20Base%20Object%20Reference) (UnlockSound :type Sound%20Base%20Object%20Reference) (Location :type Vector))
  (if (not (Variables|Default|GetStop))
    (if (Variables|Default|GetIsLocked)
      (bind _has_ (Default|HasItem (Variables|Default|GetBP%20Inventory%20Component) (Variables|Default|GetKeyID)))
      (if _has_
        (Variables|Default|SetStop true)
        (Utilities|IsValid UnlockSound
          (:Is%20Valid
            (bind _returnvalue (Audio|SpawnSoundatLocation UnlockSound Location "0, 0, 0" 1.0 1.0 0.0 "/Game/Audio/Doors/Door_Attenuation.Door_Attenuation" 0))
            (Utilities|FlowControl|Delay (Variables|/Script/Engine.SoundBase|GetDuration (Variables|/Script/Engine.AudioComponent|GetSound _returnvalue))))
          (:Is%20Not%20Valid
            (bind _returnvalue_2 (Audio|SpawnSoundatLocation (Variables|Default|GetUnlock%20Sound) Location "0, 0, 0" 1.0 1.0 0.0 "/Game/Audio/Doors/Door_Attenuation.Door_Attenuation" 0))
            (Utilities|FlowControl|Delay (Variables|/Script/Engine.SoundBase|GetDuration (Variables|/Script/Engine.AudioComponent|GetSound _returnvalue_2)))))
        (Variables|Default|SetStop false)
        (Variables|Default|SetIsLocked false)
        (CallFunction|Open/CloseDoor)
        (else
          (Utilities|IsValid Jiggle%20Sound
            (:Is%20Valid
              (Audio|SpawnSoundatLocation Jiggle%20Sound Location "0, 0, 0" 1.0 1.0 0.0 "/Game/Audio/Doors/Door_Attenuation.Door_Attenuation" 0))
            (:Is%20Not%20Valid
              (Audio|SpawnSoundatLocation (Variables|Default|GetLockedSound) Location "0, 0, 0" 1.0 1.0 0.0 "/Game/Audio/Doors/Door_Attenuation.Door_Attenuation" 0)))))
      (else
        (CallFunction|Open/CloseDoor)))))

(event EventBeginPlay
  (|CallParentFunction)
  (bind _asbp_first_person_character (Utilities|Casting|CastToBP_FirstPersonCharacter (Game|GetPlayerCharacter 0)))
  (Variables|Default|SetBP%20Inventory%20Component (Variables|/Game/BP/Character/BP_FirstPersonCharacter.BP_FirstPersonCharacter_C|GetBP_InventoryComponent _asbp_first_person_character)))

(event Collision|EventActorBeginOverlap
  (params (OtherActor :type Actor%20Object%20Reference))
  (|CallParentFunction OtherActor) ; This node is disabled and will not be called.\nDrag off pins to build functionality.
)

(event EventTick
  (params (DeltaSeconds :type Float%20%28single-precision%29))
  (|CallParentFunction DeltaSeconds) ; This node is disabled and will not be called.\nDrag off pins to build functionality.
)

(fn ConstructionScript
  (|CallParentFunction))