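; Child Blueprint of the locked door base, an interactable door that tries to open when the player interacts with it.
; BeginPlay runs the parent setup, then calls setters for timeline play rate, open and close sounds, open angle and optional close-sound delay, with zero or unset values.
; Interact passes the root component's world location to TryOpenDoor, leaving the door logic to inherited functions.
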(event EventBeginPlay
  (|CallParentFunction)
  ;[0.15 0.15 0.15 0.5] Door Settings
  (CallFunction|SetTLPlayRate 0.0)
  (CallFunction|SetOpenandCloseSounds)
  (CallFunction|SetOpenAngle 0.0)
  ;;[0.15 0.15 0.15 0.5] Optional
  (CallFunction|SetCloseSoundDelay 0.0))

(event Collision|EventActorBeginOverlap
  (params (OtherActor :type Actor%20Object%20Reference))
  (|CallParentFunction OtherActor) ; This node is disabled and will not be called.\nDrag off pins to build functionality.
)

(event EventTick
  (params (DeltaSeconds :type Float%20%28single-precision%29))
  (|CallParentFunction DeltaSeconds) ; This node is disabled and will not be called.\nDrag off pins to build functionality.
)

(event EventInteract
  (CallFunction|TryOpenDoor 0 0 (Transformation|GetWorldLocation (Variables|Default|GetDefaultSceneRoot))))

(fn ConstructionScript
  (|CallParentFunction))