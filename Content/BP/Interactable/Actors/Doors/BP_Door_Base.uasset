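; Base interactable door that toggles open and closed on interaction, updating its prompt text to match.
; Interact calls a toggle that plays or reverses a timeline, lerping door yaw from its starting rotation by OpenAngle.
; CanInteract blocks re-triggering until a short delay from timeline updates clears it, while positional sounds play, the close one delayed.
; Guarded setters configure play rate, angle, sound delay and sounds.
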(event Custom|Open/Close%20Door
  (bind _startingrotation (Variables|Default|GetStartingRotation))
  (bind _defaultsceneroot (Variables|Default|GetDefaultSceneRoot))
  (bind _returnvalue (Transformation|GetWorldLocation _defaultsceneroot))
  ;[0.15 0.15 0.15 0.5] Interaction Override
  (if (Variables|Default|GetCanInteract)
    (Variables|Default|SetCanInteract false)
    (if (Variables|Default|GetIs%20Opened)
      (Variables|Default|SetIs%20Opened false)
      (Utilities|FlowControl|Sequence
        (:then_0
          (bind _alpha (Timeline|DoorTL Reverse)
            (:Update
              (Transformation|SetRelativeRotation (Variables|Components|GetDoor) (Math|Rotator|MakeRotator (.roll _startingrotation) (.pitch _startingrotation) (Math|Float|Lerp (.yaw _startingrotation) (- (.yaw _startingrotation) (Variables|Default|GetOpenAngle)) _alpha)) false false)
              (Utilities|FlowControl|Delay 0.2)
              (Variables|Default|SetCanInteract true))))
        (:then_1
          (Utilities|FlowControl|Delay (Variables|Default|GetCloseSoundDelay))
          (Audio|SpawnSoundatLocation (Variables|Default|GetClose%20Sound) _returnvalue "0, 0, 0" 1.0 1.0 0.0 (Variables|Default|GetAttenuation%20Settings) 0)
          (Utilities|FlowControl|Delay 0.2)
          (CallFunction|SetInteractionText "Press E to Open")))
      (else
        (Variables|Default|SetIs%20Opened true)
        (Utilities|FlowControl|Sequence
          (:then_0
            (Timeline|DoorTL Play))
          (:then_1
            (Audio|SpawnSoundatLocation (Variables|Default|GetOpen%20Sound) _returnvalue "0, 0, 0" 1.0 1.0 0.0 (Variables|Default|GetAttenuation%20Settings) 0)
            (Utilities|FlowControl|Delay 0.2)
            (CallFunction|SetInteractionText "Press E to Close")))))))

(event EventBeginPlay
  (|CallParentFunction)
  ;[0.15 0.15 0.15 0.5] Custom Interaction Text
  (CallFunction|SetInteractionText "Press E to Open")
  (Variables|Default|SetStartingRotation (Variables|/Script/Engine.SceneComponent|GetRelativeRotation (Variables|Components|GetDoorBase))))

(event Collision|EventActorBeginOverlap
  (params (OtherActor :type Actor%20Object%20Reference))
  (|CallParentFunction OtherActor) ; This node is disabled and will not be called.\nDrag off pins to build functionality.
)

(event EventTick
  (params (DeltaSeconds :type Float%20%28single-precision%29))
  (|CallParentFunction DeltaSeconds) ; This node is disabled and will not be called.\nDrag off pins to build functionality.
)

(event EventInteract
  ;[0.15 0.15 0.15 0.5] Interaction Override
  (CallFunction|Open/CloseDoor))

(fn ConstructionScript
  (|CallParentFunction))

(fn SetTLPlayRate
  (params (Play%20Rate :type Float%20%28double-precision%29))
  (if (!= Play%20Rate 0.0)
    (bind _output_get (Variables|Default|SetTL%20Play%20Rate Play%20Rate))
    (Components|Timeline|SetPlayRate (Variables|Default|GetDoorTL) _output_get)))

(fn SetOpenAngle
  (params (Angle :type Float%20%28double-precision%29))
  (if (and (!= Angle 0.0) (<= Angle 1.8e+02))
    (Variables|Default|SetOpenAngle Angle)))

(fn SetCloseSoundDelay
  (params (Delay :type Float%20%28double-precision%29))
  (if (!= Delay 0.0)
    (Variables|Default|SetCloseSoundDelay Delay)))

(fn SetOpenandCloseSounds
  (params (OpenSound :type Sound%20Base%20Object%20Reference) (CloseSound :type Sound%20Base%20Object%20Reference))
  (Utilities|IsValid OpenSound
    (:Is%20Valid
      (Variables|Default|SetOpen%20Sound OpenSound))
    (:Is%20Not%20Valid
      _))
  (Utilities|IsValid CloseSound
    (:Is%20Valid
      (Variables|Default|SetClose%20Sound CloseSound))))