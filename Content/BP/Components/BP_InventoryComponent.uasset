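; BP_InventoryComponent is an inventory component that stores items in an array and provides add, remove and lookup functions.
; AddItem rejects an item flagged unique if its ID is already held, playing an error sound; otherwise it appends it.
; RemoveItem deletes an item if present, and both it and AddItem return success as a boolean.
; HasItem scans by ItemID, breaking on the first match.
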(fn AddItem
  (params (New%20Item :type Item%20Struct%20Structure))
  (bind (_itemid _itemname _usunique) (Utilities|Struct|BreakItemStruct New%20Item))
  (if _usunique
    (bind _has_ (CallFunction|HasItem _itemid))
    (if _has_
      (Audio|PlaySound2D "/Game/Audio/Effects/errEffect.errEffect" 1.0 1.0 0.0 0 0 false)
      (return false)
      (else
        _)))
  (Utilities|Array|Add (Variables|Default|GetInventory) New%20Item)
  (return true))

(fn RemoveItem
  (params (Item :type Item%20Struct%20Structure%20%28by%20ref%29))
  (bind _inventory (Variables|Default|GetInventory))
  (if (Utilities|Array|ContainsItem _inventory Item)
    (Utilities|Array|RemoveItem _inventory Item)
    (return true)
    (else
      (return false))))

(fn HasItem
  (params (ItemID :type String))
  (bind _array_element (Utilities|Array|ForEachLoopwithBreak (Variables|Default|GetInventory) :!label _label)
    (:LoopBody
      (if (Utilities|Enum|Equal(Enum) ItemID (.ItemID (Utilities|Struct|BreakItemStruct _array_element)))
        (goto _label Break)))
    (:Completed
      (return (Utilities|Enum|Equal(Enum) ItemID (.ItemID (Utilities|Struct|BreakItemStruct _array_element)))))))